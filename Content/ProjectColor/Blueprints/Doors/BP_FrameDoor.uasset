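; BP_FrameDoor is a door actor that swings open by rotating its root scene component around the yaw axis.
; BeginPlay runs the parent logic, then caches the root's starting relative yaw.
; The OpenDoor event plays a timeline whose ZRotation track is added to that cached yaw, leaving roll and pitch unchanged, so the swing is relative to the door's initial orientation.
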(event EventOpenDoor
  (bind _rootscene (Variables|Default|GetRootScene))
  (bind _relativerotation (Variables|/Script/Engine.SceneComponent|GetRelativeRotation _rootscene))
  (bind _zrotation (Timeline|Timeline Play)
    (:Update
      (Transformation|SetRelativeRotation (Variables|Default|GetRootScene) (Math|Rotator|MakeRotator (.roll _relativerotation) (.pitch _relativerotation) (+ _zrotation (Variables|Default|GetInitialZRotation))) false false))))

(event EventBeginPlay
  (|CallParentFunction)
  (Variables|Default|SetInitialZRotation (.yaw (Variables|/Script/Engine.SceneComponent|GetRelativeRotation (Variables|Default|GetRootScene)))))

(fn ConstructionScript)
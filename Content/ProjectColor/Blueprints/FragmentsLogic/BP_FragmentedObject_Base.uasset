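; Base Blueprint for fragmented puzzle objects that plays the resolution sequence when their puzzle is solved.
; ResolutionStart plays a sound and runs a timeline that rebuilds the fragments at their origin.
; It then moves the object along a spline before calling PuzzleResolved, while ColorRoomStart recolors the room in parallel.
; Recoloring casts self to Rocket, Cake or Grammophone to animate that level's MPC_ProjectColor parameter, skipping Key.
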(event EventColorRoomStart
  (bind _self self)
  ;[0.15 0.15 0.15 0.5] Aggiunge la logica di ricolorazione di tutte le stanze
  (Utilities|Casting|CastToBP_Key _self
    (:CastFailed
      (Utilities|Casting|CastToBP_Rocket _self
        (:then
          (Components|Timeline|SetPlayRate (Variables|Default|GetTimeline_ColorLevel1) (/ 1.0 (Variables|Default|GetTimeToRecolorRoom)))
          (bind _from_bw_to_color (Timeline|Timeline_ColorLevel1 Play)
            (:Update
              (Rendering|Material|SetScalarParameterValue "/Game/ProjectColor/Materials/BlackAndWhite/MPC_ProjectColor.MPC_ProjectColor" "NoColorLevel1" _from_bw_to_color :!class /Script/Engine.KismetMaterialLibrary))))
        (:CastFailed
          (Utilities|Casting|CastToBP_Cake _self
            (:then
              (Components|Timeline|SetPlayRate (Variables|Default|GetTimeline_ColorLevel2) (/ 1.0 (Variables|Default|GetTimeToRecolorRoom)))
              (bind _from_bw_to_color_2 (Timeline|Timeline_ColorLevel2 Play)
                (:Update
                  (Rendering|Material|SetScalarParameterValue "/Game/ProjectColor/Materials/BlackAndWhite/MPC_ProjectColor.MPC_ProjectColor" "NoColorLevel2" _from_bw_to_color_2 :!class /Script/Engine.KismetMaterialLibrary))))
            (:CastFailed
              (Utilities|Casting|CastToBP_Grammophone _self)
              (Components|Timeline|SetPlayRate (Variables|Default|GetTimeline_ColorLevel3) (/ 1.0 (Variables|Default|GetTimeToRecolorRoom)))
              (bind _from_bw_to_color_3 (Timeline|Timeline_ColorLevel3 Play)
                (:Update
                  (Rendering|Material|SetScalarParameterValue "/Game/ProjectColor/Materials/BlackAndWhite/MPC_ProjectColor.MPC_ProjectColor" "NoColorLevel3" _from_bw_to_color_3 :!class /Script/Engine.KismetMaterialLibrary))))))))))

(event EventResolutionStart
  (Class|FragmentedObject|PlayPuzzleResolvedSound)
  ;[0.15 0.15 0.15 0.5] Move fragments to origin / object rebuilding animation
  (Components|Timeline|SetPlayRate (Variables|Default|GetMoveFragmentsToOriginTimeline) (/ 1.0 (Variables|Default|GetTimeToRebuildObject)))
  (bind _alpha (Timeline|MoveFragmentsToOriginTimeline Play)
    (:Update
      (Class|FragmentedObject|MoveFragmentstoOrigin _alpha))
    (:Finished
      (Class|FragmentedObject|ColorRoomStart)
      ;[0.15 0.15 0.15 0.5] Move object to end location along spline
      (Components|Timeline|SetPlayRate (Variables|Default|GetMoveObjectToEndLocationTimeline) (/ 1.0 (Variables|Default|GetTimeToCompleteSplineMovement)))
      (bind _alpha_2 (Timeline|MoveObjectToEndLocationTimeline Play)
        (:Update
          (Class|FragmentedObject|MoveObjecttoEndLocation _alpha_2))
        (:Finished
          (Class|FragmentedObject|PuzzleResolved true))))))

(fn ConstructionScript)